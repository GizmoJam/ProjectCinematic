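; Tram actor for the sci-fi station, with sliding front and back doors that open automatically for the first-person character.
; Overlapping either door trigger plays that set's timeline, sliding four door meshes along local X using mirrored Left/Right tracks.
; When a timeline finishes, a short retriggerable delay precedes reversing it to close the doors.
; Back doors move through the OpenDoor function, while front doors set their locations inline.
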(event `self.doors_a.OnComponentBeginOverlap`
  (params (OverlappedComponent :type "PrimitiveComponent Object Reference") (OtherActor :type "Actor Object Reference") (OtherComp :type "PrimitiveComponent Object Reference") (OtherBodyIndex :type Integer) (bFromSweep :type Boolean) (SweepResult :type "HitResult Structure (by ref)"))
  (cast `/Game/SciFiTramStation/EpicContent/FirstPerson/FirstPersonBP/Blueprints/FirstPersonCharacter` OtherActor)
  (`|ExecutionSequence`
    (:`then_0`
      ;[0 0.3616 1] Back doors
      ;;[1 1 1] Doors Opening
      (bind (_direction _right _left) (`Timeline|Movement` :!label _label)
        (:`Update`
          (`self.OpenDoor` _right _left _right _left))
        (:`Finished`
          (if true
            (`KismetSystemLibrary.RetriggerableDelay` 2.0)
            (goto _label :!via `Reverse`)))))))

(event `self.doors_b.OnComponentBeginOverlap`
  (params (OverlappedComponent :type "PrimitiveComponent Object Reference") (OtherActor :type "Actor Object Reference") (OtherComp :type "PrimitiveComponent Object Reference") (OtherBodyIndex :type Integer) (bFromSweep :type Boolean) (SweepResult :type "HitResult Structure (by ref)"))
  (bind _sm_tram_door_left3 (`self.SM_Tram_Door_Left3`))
  (bind _sm_tram_door_right2 (`self.SM_Tram_Door_Right2`))
  (bind _sm_tram_door_left2 (`self.SM_Tram_Door_Left2`))
  (bind _sm_tram_door_right3 (`self.SM_Tram_Door_Right3`))
  (bind (_relativelocation_x _relativelocation_y _relativelocation_z) (`KismetMathLibrary.BreakVector` (`SceneComponent.RelativeLocation` _sm_tram_door_right3)))
  (bind (_relativelocation_x_2 _relativelocation_y_2 _relativelocation_z_2) (`KismetMathLibrary.BreakVector` (`SceneComponent.RelativeLocation` _sm_tram_door_left3)))
  (bind (_relativelocation_x_3 _relativelocation_y_3 _relativelocation_z_3) (`KismetMathLibrary.BreakVector` (`SceneComponent.RelativeLocation` _sm_tram_door_right2)))
  (bind (_relativelocation_x_4 _relativelocation_y_4 _relativelocation_z_4) (`KismetMathLibrary.BreakVector` (`SceneComponent.RelativeLocation` _sm_tram_door_left2)))
  (cast `/Game/SciFiTramStation/EpicContent/FirstPerson/FirstPersonBP/Blueprints/FirstPersonCharacter` OtherActor)
  (`|ExecutionSequence`
    (:`then_0`
      ;[1 0 0] Front doors
      ;;[1 1 1] Doors2 Opening
      (bind (_direction _right _left) (`Timeline|Movement2` :!label _label_2)
        (:`Update`
          (`SceneComponent.K2_SetRelativeLocation` _sm_tram_door_left2 (`KismetMathLibrary.MakeVector` _left _relativelocation_y_4 _relativelocation_z_4) false false)
          (`SceneComponent.K2_SetRelativeLocation` _sm_tram_door_right2 (`KismetMathLibrary.MakeVector` _right _relativelocation_y_3 _relativelocation_z_3) false false)
          (`SceneComponent.K2_SetRelativeLocation` _sm_tram_door_left3 (`KismetMathLibrary.MakeVector` _right _relativelocation_y_2 _relativelocation_z_2) false false)
          (`SceneComponent.K2_SetRelativeLocation` _sm_tram_door_right3 (`KismetMathLibrary.MakeVector` _left _relativelocation_y _relativelocation_z) false false))
        (:`Finished`
          (if true
            (`KismetSystemLibrary.RetriggerableDelay` 2.0)
            (goto _label_2 :!via `Reverse`)))))))

(fn `OpenDoor`
  (params (NewLocation_X :type "Float (double-precision)") (NewLocation_X2 :type "Float (double-precision)") (NewLocation_X3 :type "Float (double-precision)") (NewLocation_X4 :type "Float (double-precision)"))
  (bind _sm_tram_door_left (`self.SM_Tram_Door_Left`))
  (bind _sm_tram_door_right1 (`self.SM_Tram_Door_Right1`))
  (bind _sm_tram_door_left1 (`self.SM_Tram_Door_Left1`))
  (bind _sm_tram_door_right (`self.SM_Tram_Door_Right`))
  (bind (_relativelocation_x _relativelocation_y _relativelocation_z) (`KismetMathLibrary.BreakVector` (`SceneComponent.RelativeLocation` _sm_tram_door_right)))
  (bind (_relativelocation_x_2 _relativelocation_y_2 _relativelocation_z_2) (`KismetMathLibrary.BreakVector` (`SceneComponent.RelativeLocation` _sm_tram_door_left)))
  (bind (_relativelocation_x_3 _relativelocation_y_3 _relativelocation_z_3) (`KismetMathLibrary.BreakVector` (`SceneComponent.RelativeLocation` _sm_tram_door_left1)))
  (bind (_relativelocation_x_4 _relativelocation_y_4 _relativelocation_z_4) (`KismetMathLibrary.BreakVector` (`SceneComponent.RelativeLocation` _sm_tram_door_right1)))
  (`SceneComponent.K2_SetRelativeLocation` _sm_tram_door_left (`KismetMathLibrary.MakeVector` NewLocation_X2 _relativelocation_y_2 _relativelocation_z_2) false false)
  (`SceneComponent.K2_SetRelativeLocation` _sm_tram_door_right (`KismetMathLibrary.MakeVector` NewLocation_X _relativelocation_y _relativelocation_z) false false)
  (`SceneComponent.K2_SetRelativeLocation` _sm_tram_door_right1 (`KismetMathLibrary.MakeVector` NewLocation_X4 _relativelocation_y_4 _relativelocation_z_4) false false)
  (`SceneComponent.K2_SetRelativeLocation` _sm_tram_door_left1 (`KismetMathLibrary.MakeVector` NewLocation_X3 _relativelocation_y_3 _relativelocation_z_3) false false))

(fn `UserConstructionScript`)