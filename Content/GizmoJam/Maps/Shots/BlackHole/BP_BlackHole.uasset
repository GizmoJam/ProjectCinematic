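; BP_BlackHole is a placeable black hole visual whose look is tuned through exposed Blueprint variables.
; Its construction script pushes color, emissive, size, horizon, ring and Doppler values into material parameters on the BH component.
; The effect itself lives in that material, as the event graph holds only disabled default nodes and no runtime logic.
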(fn `UserConstructionScript`
  (`MeshComponent.SetScalarParameterValueOnMaterials` (`self.BH`) "Emissive int" (`self.Emissive int`))
  (`MeshComponent.SetVectorParameterValueOnMaterials` (`self.BH`) "Color Black Hole" (`self.Color`))
  (`MeshComponent.SetScalarParameterValueOnMaterials` (`self.BH`) "Black hole size" (`self.Black hole size`))
  (`MeshComponent.SetScalarParameterValueOnMaterials` (`self.BH`) "Step" (`self.Step`))
  (`MeshComponent.SetScalarParameterValueOnMaterials` (`self.BH`) "Horizont_size" (`self.Horizont_size`))
  (`MeshComponent.SetScalarParameterValueOnMaterials` (`self.BH`) "rv" (`self.rv`))
  (`MeshComponent.SetScalarParameterValueOnMaterials` (`self.BH`) "rrad" (`self.rrad`))
  (`MeshComponent.SetScalarParameterValueOnMaterials` (`self.BH`) "Ring_Radius" (`self.Ring_Radius`))
  (`MeshComponent.SetScalarParameterValueOnMaterials` (`self.BH`) "Texture_Stretch" (`self.Texture_Stretch`))
  (`MeshComponent.SetScalarParameterValueOnMaterials` (`self.BH`) "Doppler_int" (`self.Doppler_int`))
  (`MeshComponent.SetScalarParameterValueOnMaterials` (`self.BH`) "maxrot" (`self.maxrot`))
  (`MeshComponent.SetScalarParameterValueOnMaterials` (`self.BH`) "Ring_speed" (`self.Ring_speed`))
  (`MeshComponent.SetScalarParameterValueOnMaterials` (`self.BH`) "Ring_int" (`self.Ring_int`))
  (`MeshComponent.SetScalarParameterValueOnMaterials` (`self.BH`) "rint" (`self.rint`))
  (`MeshComponent.SetScalarParameterValueOnMaterials` (`self.BH`) "inring" (`self.inring`))
  (`MeshComponent.SetScalarParameterValueOnMaterials` (`self.BH`) "Ring_int_faloff" (`self.Ring_int_faloff`))
  (`MeshComponent.SetScalarParameterValueOnMaterials` (`self.BH`) "rfac" (`self.rfac`)))